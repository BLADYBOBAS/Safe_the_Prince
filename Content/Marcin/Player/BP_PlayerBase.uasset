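; Base player character for a top-down-style shooter, with control-rotation-relative movement, mouse-cursor aiming and a hitscan pistol.
; BeginPlay retries until the player character is valid, then caches it through an interface and sets up Enhanced Input, cursor and HUD.
; Tick turns the actor's yaw toward the cursor hit point, storing it as the shot direction.
; Interface-called firing spends ammo, line-traces and damages Enemy-tagged actors; ammo changes update the HUD.
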(event `self.ReceiveBeginPlay`
  (bind _returnvalue (`GameplayStatics.GetPlayerCharacter` 0))
  ;[1 0.1448 0.6305] Input
  ;;[0.05098 0.05098 0.05098] Add Mapping Context
  (`parent.ReceiveBeginPlay`)
  (`/Engine/EditorBlueprintResources/StandardMacros.IsValid` _returnvalue :!label _label
    (:`Is Valid`
      (bind _player (message `/Game/Marcin/Player/BPI_PlayerBase.PlayerRef` _returnvalue))
      (set `self.PlayerPawn` _player)
      (bind _asplayer_controller (cast `PlayerController` (`self.GetController`)))
      (bind _returnvalue_2 (pcsubsystem `EnhancedInputLocalPlayerSubsystem` _asplayer_controller))
      (`/Engine/EditorBlueprintResources/StandardMacros.IsValid` _returnvalue_2
        (:`Is Valid`
          (`EnhancedInputSubsystemInterface.AddMappingContext` _returnvalue_2 "/Game/Marcin/InputMK/IMC_MK.IMC_MK" 0 (struct))
          (set `PlayerController.bShowMouseCursor` true (`GameplayStatics.GetPlayerController` 0))
          ;[1 0.1448 0.6305] HUD
          (bind _returnvalue_3 (`|CreateWidget` "/Game/Marcin/UI/WBP_HUD.WBP_HUD_C"))
          (bind _output_get (set `self.PlayerHUDRef` _returnvalue_3))
          (`UserWidget.AddToViewport` _output_get 0))))
    (:`Is Not Valid`
      (`KismetSystemLibrary.Delay` 0.2)
      (goto _label))))

(event `EnhancedInput|/Game/Marcin/InputMK/Actions/IA_Move`
  (params (ActionValue :type "Vector2D Structure") (ElapsedSeconds :type "Float (double-precision)") (TriggeredSeconds :type "Float (double-precision)") (InputAction :type "InputAction Object Reference" :default "/Game/Marcin/InputMK/Actions/IA_Move.IA_Move"))
  (bind (_returnvalue_roll _returnvalue_pitch _returnvalue_yaw) (`KismetMathLibrary.BreakRotator` (`self.GetControlRotation`)))
  (bind (_returnvalue_roll_2 _returnvalue_pitch_2 _returnvalue_yaw_2) (`KismetMathLibrary.BreakRotator` (`self.GetControlRotation`)))
  ;[1 0.1448 0.6305] Player Controller
  (:`Triggered`
    (`self.AddMovementInput` (`KismetMathLibrary.GetRightVector` (`KismetMathLibrary.MakeRotator` _returnvalue_roll_2 0.0 _returnvalue_yaw_2)) ActionValue_X)
    (`self.AddMovementInput` (`KismetMathLibrary.GetForwardVector` (`KismetMathLibrary.MakeRotator` 0.0 0.0 _returnvalue_yaw)) ActionValue_Y)))

(event `self.ReceiveTick`
  (params (DeltaSeconds :type "Float (single-precision)"))
  (bind (_returnvalue_roll _returnvalue_pitch) (`KismetMathLibrary.BreakRotator` (`self.K2_GetActorRotation`)))
  (bind (_returnvalue_roll_2 _returnvalue_pitch_2 _returnvalue_yaw) (`KismetMathLibrary.BreakRotator` (`KismetMathLibrary.RInterpTo_Constant` (`self.K2_GetActorRotation`) (`KismetMathLibrary.FindLookAtRotation` (+ (0.0 0.0 0.0) (0.0 0.0 0.0)) (- (`.ImpactPoint` (`GameplayStatics.BreakHitResult` (`PlayerController.GetHitResultUnderCursorByChannel` (`GameplayStatics.GetPlayerController` 0) "TraceTypeQuery1" true))) (`self.K2_GetActorLocation`))) (`GameplayStatics.GetWorldDeltaSeconds`) (`self.Rotation Speed`))))
  ;[1 0.1448 0.6305] Patrzenie w kierunku kursora myszki
  (`parent.ReceiveTick` 0.0)
  (`self.K2_SetActorRotation` (`KismetMathLibrary.MakeRotator` _returnvalue_roll _returnvalue_pitch _returnvalue_yaw))
  (set `self.playerRotation` _returnvalue_yaw))

(event `EnhancedInput|/Game/Marcin/InputMK/Actions/IA_FireWeapon`
  (params (ActionValue :type Boolean) (ElapsedSeconds :type "Float (double-precision)") (TriggeredSeconds :type "Float (double-precision)") (InputAction :type "InputAction Object Reference" :default "/Game/Marcin/InputMK/Actions/IA_FireWeapon.IA_FireWeapon"))
  ;[1 0.1448 0.6305] Fire Weapon calls BP interface event
  (:`Started`
    (`self.FireWeapon` (`self.PlayerPawn`))))

(event `/Game/Marcin/Player/BPI_PlayerBase.FireWeapon`
  (bind _bulletspawner (`self.BulletSpawner`))
  (bind (_worldlocation _worldrotation) (`self.GetBulletSpawnLocAndRot` _bulletspawner))
  ;[1 0.1448 0.6305] Fire Weapon
  (if (>= (`self.Ammo`) 1)
    (bind _output_get (set `self.Ammo` (- (`self.Ammo`) 1)))
    (`/Game/Marcin/UI/WBP_HUD.UpdateAmmo` (`self.PlayerHUDRef`))
    (`KismetSystemLibrary.PrintString` (`KismetStringLibrary.Conv_IntToString` _output_get))
    (`GameplayStatics.SpawnEmitterAttached` "/Game/Marcin/MilitaryWeapDark/FX/P_Pistol_MuzzleFlash_01.P_Pistol_MuzzleFlash_01" _bulletspawner "None" _worldlocation (`KismetMathLibrary.Conv_VectorToRotator` _worldrotation) (1.0 1.0 1.0) "KeepWorldPosition")
    (`GameplayStatics.PlaySoundAtLocation` "/Game/Marcin/MilitaryWeapDark/Sound/Pistol/PistolB_Fire_Cue.PistolB_Fire_Cue" _worldlocation (struct) 1.0 1.0 0.0 null null null null)
    (bind _outhit (`KismetSystemLibrary.LineTraceSingle` :`Start` _worldlocation :`End` (+ _worldlocation (* _worldrotation (`self.BulletDistance`))) :`TraceChannel` "TraceTypeQuery1" :`DrawDebugType` "ForOneFrame"))
    (bind (_bblockinghit _binitialoverlap _time _distance _location _impactpoint _normal _impactnormal _physmat _hitactor) (`GameplayStatics.BreakHitResult` _outhit))
    (if (`self.ActorHasTag` _hitactor "Enemy")
      (`GameplayStatics.PlaySoundAtLocation` "/Game/Marcin/MilitaryWeapDark/Sound/Knife/Knife_ImpactBody_Cue.Knife_ImpactBody_Cue" _location (struct) 1.0 1.0 0.0 null null null null)
      (`GameplayStatics.ApplyDamage` _hitactor (`KismetMathLibrary.Conv_IntToDouble` (`self.BulletDamage`)) (`GameplayStatics.GetPlayerController` 0) self))
    (else
      (`GameplayStatics.PlaySoundAtLocation` "/Game/Marcin/MilitaryWeapDark/Sound/Pistol/Pistol_MagEject_Cue.Pistol_MagEject_Cue" (`self.GetBulletSpawnLocAndRot` (`self.BulletSpawner`)) (struct) 1.0 1.0 0.0 null null null null))))

(event `AddAmmo`
  (params (AmmoToAdd :type Integer))
  (set `self.Ammo` (`KismetMathLibrary.Clamp` (+ AmmoToAdd (`self.Ammo`)) 0 (`self.MaxAmmo`)))
  (`/Game/Marcin/UI/WBP_HUD.UpdateAmmo` (`self.PlayerHUDRef`)))

(fn `GetBulletSpawnLocAndRot`
  (params (Object :type "SceneComponent Object Reference"))
  (returns (worldLocation :type "Vector Structure") (worldRotation :type "Vector Structure"))
  (return (`SceneComponent.K2_GetComponentLocation` Object) (`KismetMathLibrary.GetForwardVector` (`KismetMathLibrary.MakeRotator` 0.0 0.0 (`self.playerRotation`)))))

(fn `PlayerRef`
  (returns (Player :type "/Game/Marcin/Player/BP_PlayerBase Object Reference"))
  (return self))

(fn `UserConstructionScript`
  (`parent.UserConstructionScript`))