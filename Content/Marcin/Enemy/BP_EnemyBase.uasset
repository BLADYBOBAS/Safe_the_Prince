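; Base enemy character that wanders the navmesh, chases the player on sight, damages them on contact and ragdolls on death.
; Wandering picks random nearby points after random pauses until PawnSensing spots the player, cached at BeginPlay with a retrying cast.
; Each sighting restarts a retriggerable delay that returns it to wandering.
; Lethal damage calls EnemyDeath, which notifies ABP_EnemyWar, disables movement and capsule collision, and enables mesh physics.
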(event `MoveAroundMap`
  ;[1 0.1448 0.6305] Random Movement
  (bind _randomlocation (`NavigationSystemV1.K2_GetRandomLocationInNavigableRadius` (`self.K2_GetActorLocation`) 1000.0 null null :!label _label))
  (`|AIMoveTo` self _randomlocation null
    (:`then`
      (`KismetSystemLibrary.Delay` (`KismetMathLibrary.RandomFloatInRange` 0.5 4.0))
      (if (not (`self.SeePlayer`))
        (goto _label)))))

(event `self.ReceiveBeginPlay`
  ;[1 0.1448 0.6305] Reference to character
  (bind _asbp_player_base (cast `/Game/Marcin/Player/BP_PlayerBase` (`GameplayStatics.GetPlayerCharacter` 0) :!label _label_2)
    (:`then`
      (set `self.As BP Player Base` _asbp_player_base)
      (goto _label))
    (:`CastFailed`
      (`KismetSystemLibrary.Delay` 0.2)
      (goto _label_2))))

(event `self.ReceiveAnyDamage`
  (params (Damage :type "Float (single-precision)") (DamageType :type "DamageType Object Reference") (InstigatedBy :type "Controller Object Reference") (DamageCauser :type "Actor Object Reference"))
  ;[1 0.1448 0.6305] Getting Hit and die
  (bind _output_get (set `self.HealthPoints` (- (`self.HealthPoints`) Damage)))
  (if (<= _output_get 0)
    (`self.EnemyDeath`)))

(event `self.PawnSensing.OnSeePawn`
  (params (Pawn :type "Pawn Object Reference"))
  (bind _as_bp_player_base (`self.As BP Player Base`))
  ;[1 0.1448 0.6305] AI Goni gracza
  (if (== Pawn _as_bp_player_base)
    (set `self.SeePlayer` true)
    (`|AIMoveTo` self (0.0 0.0 0.0) _as_bp_player_base
      (:`then`
        (`KismetSystemLibrary.RetriggerableDelay` 3.0)
        (set `self.SeePlayer` false)
        (`self.MoveAroundMap`)))))

(event `self.CapsuleComponent.OnComponentHit`
  (params (HitComponent :type "PrimitiveComponent Object Reference") (OtherActor :type "Actor Object Reference") (OtherComp :type "PrimitiveComponent Object Reference") (NormalImpulse :type "Vector Structure") (Hit :type "HitResult Structure (by ref)"))
  (bind _as_bp_player_base (`self.As BP Player Base`))
  ;[1 0.1448 0.6305] Atak na gracza
  (if (== OtherActor _as_bp_player_base)
    (`GameplayStatics.ApplyDamage` _as_bp_player_base (`self.Damage`) null self)))

(fn `EnemyDeath`
  (bind _asbp_enemy_base (cast `/Game/Marcin/Enemy/BP_EnemyBase` self))
  (bind _asabp_enemy_war (cast `/Game/Marcin/Enemy/ABP_EnemyWar` (`SkeletalMeshComponent.GetAnimInstance` (`Character.Mesh` _asbp_enemy_base))))
  (`/Game/Marcin/Enemy/ABP_EnemyWar.Died` _asabp_enemy_war)
  (`CharacterMovementComponent.DisableMovement` (`self.CharacterMovement`))
  (`PrimitiveComponent.SetSimulatePhysics` (`self.Mesh`) true)
  (`PrimitiveComponent.SetCollisionProfileName` (`self.Mesh`) "Ragdoll" true)
  (`PrimitiveComponent.SetCollisionEnabled` (`self.CapsuleComponent`) "NoCollision"))

(fn `UserConstructionScript`
  (`parent.UserConstructionScript`))